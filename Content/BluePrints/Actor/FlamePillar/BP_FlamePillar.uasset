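; BP_FlamePillar is a flame pillar actor whose light flickers continuously.
; On BeginPlay it randomly picks one of two flame intensity timelines, and each timeline picks again when it finishes, forming an endless varied loop.
; Each timeline update feeds ScaleFlameIntensity, which multiplies the curve value by BaseIntensity and applies it to the FlameLight component.
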(event Custom|StartFlameLight_1
  (bind _flameintensity (Timeline|FlameIntensity_1 PlayFromStart)
    (:Update
      (CallFunction|ScaleFlameIntensity _flameintensity))
    (:Finished
      (CallFunction|ChooseFlameTimeline))))

(event Custom|StartFlameLight_2
  (bind _flameintensity (Timeline|FlameIntensity_2 PlayFromStart)
    (:Update
      (CallFunction|ScaleFlameIntensity _flameintensity))
    (:Finished
      (CallFunction|ChooseFlameTimeline))))

(event Custom|ChooseFlameTimeline
  (switch int (Math|Random|RandomIntegerinRange 0 1)
    (:Default
      (CallFunction|StartFlameLight2 :!label _label))
    (:0
      (CallFunction|StartFlameLight1))
    (:1
      (goto _label))))

(event EventBeginPlay
  (CallFunction|ChooseFlameTimeline))

(event Collision|EventActorBeginOverlap
  (params (OtherActor :type Actor%20Object%20Reference)))

(event EventTick
  (params (DeltaSeconds :type Float%20%28single-precision%29)))

(fn ConstructionScript)

(fn ScaleFlameIntensity
  (params (Intensity :type Float%20%28double-precision%29))
  (Rendering|Components|Light|SetIntensity (Variables|Default|GetFlameLight) (* Intensity (Variables|Default|GetBaseIntensity))))