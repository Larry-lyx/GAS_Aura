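; BP_FadeActor is a static mesh actor that fades out and back in through a material "Fade" parameter.
; The construction script caches original materials and builds dynamic instances from FadeMaterialInstances, which FadeOut swaps onto the mesh.
; A timeline drives the parameter, and Fadein reverses it.
; On finish, Fade at 1 restores original materials and blocking, while 0 ignores a custom trace channel and, optionally, Visibility.
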(event Collision|EventActorBeginOverlap
  (params (OtherActor :type Actor%20Object%20Reference)))

(event EventTick
  (params (DeltaSeconds :type Float%20%28single-precision%29)))

(event EventFadeOut
  (CallFunction|SetMaterialtoDynamicInstances)
  (bind _fade (Timeline|FadeTImeline Play)
    (:Update
      (for _array_element (Variables|Default|GetDynamicMaterials)
        (Rendering|Material|SetScalarParameterValue _array_element "Fade" _fade :!class /Script/Engine.MaterialInstanceDynamic)))
    (:Finished
      (CallFunction|FadeFinished _fade))))

(event EventFadein
  (bind _fade (Timeline|FadeTImeline Reverse)
    (:Update
      (for _array_element (Variables|Default|GetDynamicMaterials)
        (Rendering|Material|SetScalarParameterValue _array_element "Fade" _fade :!class /Script/Engine.MaterialInstanceDynamic)))
    (:Finished
      (CallFunction|FadeFinished _fade))))

(fn ConstructionScript
  (Utilities|Array|Clear (Variables|Default|GetDynamicMaterials))
  (Variables|Default|SetOriginalMaterials (Rendering|Material|GetMaterials (Variables|Default|GetStaticMesh)))
  (for _array_element (Variables|Default|GetFadeMaterialInstances)
    (bind _returnvalue (Rendering|Material|CreateDynamicMaterialInstance _array_element "None" "None" :!class /Script/Engine.KismetMaterialLibrary))
    (Utilities|Array|AddUnique (Variables|Default|GetDynamicMaterials) _returnvalue)))

(fn SetMaterialtoDynamicInstances
  (for (_array_element _array_index) (Variables|Default|GetDynamicMaterials)
    (Rendering|Material|SetMaterial (Variables|Default|GetStaticMesh) _array_index _array_element)))

(fn ResetMaterials
  (for (_array_element _array_index) (Variables|Default|GetOriginalMaterials)
    (Rendering|Material|SetMaterial (Variables|Default|GetStaticMesh) _array_index _array_element)))

(fn FadeFinished
  (params (InputPin :type Float%20%28single-precision%29))
  (if (>= InputPin 1.0)
    (CallFunction|ResetMaterials)
    (Collision|SetCollisionResponsetoChannel (Variables|Default|GetStaticMesh) "ECC_GameTraceChannel2" "ECR_Block")
    (if (Variables|Default|GetShouldBlockVisibility)
      (Collision|SetCollisionResponsetoChannel (Variables|Default|GetStaticMesh) "ECC_Visibility" "ECR_Block"))
    (elif (<= InputPin 0.0)
      (Collision|SetCollisionResponsetoChannel (Variables|Default|GetStaticMesh) "ECC_GameTraceChannel2" "ECR_Ignore")
      (if (Variables|Default|GetShouldBlockVisibility)
        (Collision|SetCollisionResponsetoChannel (Variables|Default|GetStaticMesh) "ECC_Visibility" "ECR_Ignore")))))