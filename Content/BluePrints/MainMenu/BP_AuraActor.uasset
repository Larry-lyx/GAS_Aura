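; BP_AuraActor is the main menu scene actor that opens the menu and animates its decorative fireball and magic circle.
; On BeginPlay it plays the menu music, adds WBP_MainMenu to the viewport and switches to UI-only input with a visible cursor.
; Each Tick bobs the fireball vertically around its starting location via SinTime, which accumulates time for a scaled sine, and rolls the magic circle at a frame-rate-independent rate.
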(event EventBeginPlay
  (bind _returnvalue (Game|GetPlayerController 0))
  (Variables|Default|SetFireBallInitialLocation (Transformation|GetWorldLocation (Variables|Default|GetFireBall)))
  (bind _returnvalue_2 (Audio|SpawnSound2D "/Game/Assets/Sounds/Music/Music_MainMenu.Music_MainMenu" 1.0 1.0 0.0 0))
  (Variables|Default|SetMainMenuMusic _returnvalue_2)
  (bind _returnvalue_3 (UserInterface|CreateWidget "/Game/BluePrints/UI/MainMenu/WBP_MainMenu.WBP_MainMenu_C"))
  (UserInterface|Viewport|AddtoViewport _returnvalue_3 0)
  (Input|SetInputModeUIOnly _returnvalue 0 "DoNotLock" false)
  (Variables|/Script/Engine.PlayerController|SetbShowMouseCursor _returnvalue true))

(event Collision|EventActorBeginOverlap
  (params (OtherActor :type Actor%20Object%20Reference)))

(event EventTick
  (params (DeltaSeconds :type Float%20%28single-precision%29))
  (Transformation|SetWorldLocation (Variables|Default|GetFireBall) (+ (Variables|Default|GetFireBallInitialLocation) (Math|Vector|MakeVector 0.0 0.0 (CallFunction|SinTime DeltaSeconds))) false false)
  (Transformation|AddWorldRotation (Variables|Default|GetMagicCircle) (Math|Rotator|MakeRotator (* (Utilities|Time|GetWorldDeltaSeconds) (Variables|Default|GetMagicCircleRotationRate)) 0.0 0.0) false false))

(fn ConstructionScript)

(fn SinTime
  (params (A :type Float%20%28double-precision%29))
  (bind _output_get (Variables|Default|SetTime (+ A (Variables|Default|GetTime))))
  (return (* (Math|Trig|Sin(Radians) _output_get) (Variables|Default|GetAmplitude))))