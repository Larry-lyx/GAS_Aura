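; Fire Bolt gameplay ability that casts a projectile toward the location under the mouse.
; A target data task stores the hit location, which turns the avatar to face it through CombatInterface.
; The cast montage starts alongside a wait for its FireBolt gameplay event, which spawns the projectile from the weapon socket.
; The ability ends on a short fixed delay rather than on montage completion.
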(event Ability|EventActivateAbility
  (Utilities|FlowControl|Sequence
    (:then_0
      ;[0.15 0.15 0.15 0.5] 1. Get Projectile Target Location
      (bind _datahandle (|TargetDataUnderMouse)
        (:ValidData
          (Variables|Default|SetProjectile%20Target%20Location (.Location (Collision|BreakHitResult (Ability|TargetData|GetHitResultfromTargetData _datahandle)))))))
    (:then_1
      ;[0.15 0.15 0.15 0.5] 2. Character turn to Projectile Target
      (bind _ascombat_interface (Utilities|Casting|CastToCombatInterface (Ability|GetAvatarActorfromActorInfo)))
      (Class|CombatInterface|UpdateFacingTarget _ascombat_interface (Variables|Default|GetProjectile%20Target%20Location)))
    (:then_2
      ;[0.15 0.15 0.15 0.5] 3.Play Cast Montage and Spawn Projectile until received event notify
      (|PlayMontageandWaitProxy "None" "/Game/Assets/Characters/Aura/Animations/Abilities/AM_Cast_FireBolt.AM_Cast_FireBolt" 1.0 "None" true 1.0 0.0 false
        (:then
          (Ability|Tasks|WaitGameplayEvent "(TagName=\"Event.Montage.FireBolt\")" 0
            (:EventReceived
              (Class|AuraProjectileSpell|SpawnProjectile (Variables|Default|GetProjectile%20Target%20Location) (GameplayTags|MakeLiteralGameplayTag "(TagName=\"CombatSocket.Weapon\")")))))))
    (:then_3
      (Utilities|FlowControl|Delay 0.5)
      (Ability|EndAbility))))