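; Fireball projectile for the FireBlast ability that flies out, returns to its ReturnToActor and explodes.
; On authority, chained timelines lerp it forward to an apex, then back toward the actor's current location.
; Within ExplodeDistance it calls OnHit, applies radial damage to nearby live players except the owner, and destroys itself.
; Knockback and death impulse point away from the blast, with pitch overridden to a fixed angle.
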(event EventBeginPlay)

(event Collision|EventActorBeginOverlap
  (params (OtherActor :type Actor%20Object%20Reference)))

(event EventTick
  (params (DeltaSeconds :type Float%20%28single-precision%29)))

(event EventStartOutgoingTimeline
  (bind _returnvalue (Components|GetOwner))
  (bind _array (Utilities|Array|MakeArray _returnvalue))
  (Networking|SwitchHasAuthority
    (:Authority
      ;[0.15 0.15 0.15 0.5] Store Inital and Apex Location
      (Variables|Default|SetInitialLocation (Transformation|GetActorLocation))
      (Variables|Default|SetApexLocation (+ (Variables|Default|GetInitialLocation) (* (Transformation|GetActorForwardVector) (Variables|Default|GetTravelDistance))))
      (bind _outgoing (Timeline|OutgoingTimeline Play)
        (:Update
          (Transformation|SetActorLocation (Math|Vector|Lerp(Vector) (Variables|Default|GetInitialLocation) (Variables|Default|GetApexLocation) _outgoing) false false))
        (:Finished
          (bind _returning (Timeline|Returning%20Timeline Play)
            (:Update
              (Transformation|SetActorLocation (Math|Vector|Lerp(Vector) (Variables|Default|GetApexLocation) (Transformation|GetActorLocation (Variables|Default|GetReturnToActor)) _returning) false false)
              (if (CallFunction|IsWithinExplodeDistance)
                (Class|AuraProjectile|OnHit)
                (Utilities|Array|Add _array self)
                (bind _outoverlappingactors (Class|AuraAbilitySystemLibrary|GetLivePlayerwithRadius self _array (Variables|Default|GetRadialDamageOuterRadius) (Transformation|GetActorLocation)))
                (Variables|Default|SetOverlappingPlayers _outoverlappingactors)
                (Class|AuraAbilitySystemLibrary|SetIsRadialDamageEffectParams (Variables|Default|GetExplosionDamageParams) true (Variables|Default|GetRadialDamageInnerRadius) (Variables|Default|GetRadialDamageOuterRadius) (Transformation|GetActorLocation))
                (for _array_element (Variables|Default|GetOverlappingPlayers)
                  (Class|AuraAbilitySystemLibrary|SetEffectParamsTargetASC (Variables|Default|GetExplosionDamageParams) (Ability|GetAbilitySystemComponent _array_element))
                  (Variables|Default|SetKnockbackDirections (- (Transformation|GetActorLocation _array_element) (Transformation|GetActorLocation)))
                  (Class|AuraAbilitySystemLibrary|SetKnockbackDirection (Variables|Default|GetExplosionDamageParams) (CallFunction|OverrideKnockbackPitch) (Variables|Default|GetKnockbackMagnitude))
                  (Class|AuraAbilitySystemLibrary|SetDeathImpulseDirection (Variables|Default|GetExplosionDamageParams) (CallFunction|OverrideKnockbackPitch) (Variables|Default|GetDeathImpulseMagnitude))
                  (Class|AuraAbilitySystemLibrary|ApplyDamageEffect (Variables|Default|GetExplosionDamageParams)))
                (Actor|DestroyActor)))))))))

(fn ConstructionScript)

(fn IsWithinExplodeDistance
  (return (<= (Math|Vector|VectorLength (- (Transformation|GetActorLocation) (Transformation|GetActorLocation (Variables|Default|GetReturnToActor)))) (Variables|Default|GetExplodeDistance))))

(fn OverrideKnockbackPitch
  (bind _knockbackdirections (Variables|Default|GetKnockbackDirections))
  (bind _returnvalue (Math|Rotator|MakeRotfromX _knockbackdirections))
  (return (Math|Vector|GetForwardVector (Math|Rotator|MakeRotator (.roll _returnvalue) 45.0 (.yaw _returnvalue)))))